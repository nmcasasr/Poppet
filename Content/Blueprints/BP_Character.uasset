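; BP_Character is a character Blueprint with a sight HUD, a first- or third-person camera choice and a power-up screen effect.
; BeginPlay adds the BP_Sight widget to the viewport and caches the normal post-process settings.
; StartPowerUp applies the power-up post-process settings, and StopPowerUp restores the cached ones.
; The construction script uses UserFirstPersonView to set auto-activation on the two cameras and spring arm.
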(event EventBeginPlay
  (Utilities|FlowControl|Sequence
    (:then_0
      (bind _returnvalue (UserInterface|CreateWidget "/Game/Widgets/BP_Sight.BP_Sight_C"))
      (UserInterface|Viewport|AddtoViewport _returnvalue 0))
    (:then_1
      (Variables|Default|SetNormalPosProcessSettings (Variables|/Script/Engine.PostProcessComponent|GetSettings (Variables|Default|GetPostProcess))))))

(event EventStartPowerUp
  (Variables|/Script/Engine.PostProcessComponent|SetSettings (Variables|Default|GetPostProcess) (Variables|Default|GetPowerUpPosProcessing)))

(event EventStopPowerUp
  (Variables|/Script/Engine.PostProcessComponent|SetSettings (Variables|Default|GetPostProcess) (Variables|Default|GetNormalPosProcessSettings)))

(fn ConstructionScript
  (bind _buserfirstpersonview (Variables|Default|GetbUserFirstPersonView))
  (Components|Activation|SetAutoActivate (Variables|Default|GetTPSCameraComponent) (not _buserfirstpersonview))
  (Components|Activation|SetAutoActivate (Variables|Default|GetFPSCameraComponent) _buserfirstpersonview))