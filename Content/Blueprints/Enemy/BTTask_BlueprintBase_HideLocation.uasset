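; Behavior tree task that sends the enemy pawn to a spot 400 units from the player, on the pawn's side.
; The destination comes from the pawn-to-player direction scaled backward from the player's location, passed through a one-shot VInterpTo into AIMoveTo.
; It finishes successfully as soon as the move is issued, without waiting for arrival.
; A TargetLocation blackboard write is left unconnected.
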(event EventReceiveExecuteAI
  (params (OwnerController :type AI%20Controller%20Object%20Reference) (ControlledPawn :type Pawn%20Object%20Reference))
  (bind _returnvalue (Game|Player|GetPlayerPawn 0))
  (bind _returnvalue_2 (Transformation|GetActorLocation ControlledPawn))
  (bind _returnvalue_3 (Transformation|GetActorLocation _returnvalue))
  (AI|AIMoveTo ControlledPawn (Math|Interpolation|VInterpTo _returnvalue_2 (+ (* (Math|Vector|GetUnitDirection(Vector) _returnvalue_2 _returnvalue_3) -4e+02) _returnvalue_3) (Utilities|Time|GetWorldDeltaSeconds) 0.0) 0 5.0 false
    (:then
      (AI|BehaviorTree|FinishExecute true))))